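; Enemy-side combat component for BP_Grunt, holding health, a dead flag, attack state and montage playback for hits, counters, finishers and death.
; Taking the attack writes the blackboard AIState and registers the enemy as counter target in the player's AC_FFCC.
; Montage callbacks release the attack, randomize AI state and, for hits and counters, restart brain logic.
; Helpers compute yaw-based hit direction and teleport placement relative to the target.
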(event Custom|Play%20Hit%20Montage
  (params (Direction :type EAttackHitDirection%20Enum :default "Fwd"))
  (Animation|Montage|PlayMontage (Variables|/Script/Engine.Character|GetMesh (Variables|Default|GetOwner%20Reference)) (Utilities|Select :Index Direction :Fwd "/Game/FFCS/Blueprints/Animation/AM_Vic_1.AM_Vic_1" :Bwd "/Game/FFCS/Blueprints/Animation/MixamoUE4Model/AM_Vic_2.AM_Vic_2" :Lt "/Game/FFCS/Blueprints/Animation/MixamoUE4Model/AM_Vic_3.AM_Vic_3" :Rt "/Game/FFCS/Blueprints/Animation/MixamoUE4Model/AM_Vic_4.AM_Vic_4")
    (:then
      (bind _returnvalue (CallFunction|CheckCurrentandCounterEnemies))
      (if _returnvalue
        (CallFunction|SetAttackPlayer false)
        (CallFunction|ResetCounteredEnemyinPlayer)
        (CallFunction|SetAIStatetoRandom)
        (elif (CallFunction|GetAttackPlayer)
          (CallFunction|SetAttackPlayer false)
          (CallFunction|SetAIStatetoRandom))))
    (:OnCompleted
      (CallFunction|ControlEnemyLogic false :!label _label))
    (:OnBlendOut
      (goto _label))
    (:OnInterrupted
      (goto _label))))

(event Custom|Play%20Death%20Montage
  (bind _owner_reference (Variables|Default|GetOwner%20Reference))
  (Animation|Montage|PlayMontage (Variables|/Script/Engine.Character|GetMesh _owner_reference) "/Game/FFCS/Blueprints/Animation/AM_Death_1.AM_Death_1"
    (:then
      (CallFunction|ControlEnemyLogic true)
      (Utilities|FlowControl|Delay 5.0)
      (Actor|DestroyActor _owner_reference))))

(event Custom|PlayCounterDamage
  (params (MontageToPlay :type Anim%20Montage%20Object%20Reference))
  (Animation|Montage|PlayMontage (Variables|/Script/Engine.Character|GetMesh (Variables|Default|GetOwner%20Reference)) MontageToPlay
    (:OnCompleted
      _)
    (:OnBlendOut
      _)
    (:OnInterrupted
      _))
  (CallFunction|SetAttackPlayer false)
  (CallFunction|ResetCounteredEnemyinPlayer)
  (CallFunction|SetAIStatetoRandom)
  (CallFunction|ControlEnemyLogic false))

(event Custom|PlayFinisherMontage
  (params (MontageToPlay :type Anim%20Montage%20Object%20Reference))
  (Animation|Montage|PlayMontage (Variables|/Script/Engine.Character|GetMesh (Variables|Default|GetOwner%20Reference)) MontageToPlay
    (:OnCompleted
      _)
    (:OnBlendOut
      _)
    (:OnInterrupted
      _))
  (bind _returnvalue (CallFunction|CheckCurrentandCounterEnemies))
  (if _returnvalue
    (CallFunction|SetAttackPlayer false)
    (CallFunction|ResetCounteredEnemyinPlayer)
    (CallFunction|SetAIStatetoRandom)
    (elif (CallFunction|GetAttackPlayer)
      (CallFunction|SetAttackPlayer false)
      (CallFunction|SetAIStatetoRandom))))

(event EventBeginPlay
  (bind _asbp_grunt (Utilities|Casting|CastToBP_Grunt (Components|GetOwner)))
  (Variables|Default|SetOwner%20Reference _asbp_grunt))

(event EventTick
  (params (DeltaSeconds :type Float%20%28single-precision%29)))

(event EventSetHealth
  (params (Damage :type Float%20%28single-precision%29%20%28by%20ref%29))
  (Variables|Default|SetCurrentHealth (Math|Float|Clamp(Float) (- (CallFunction|GetHealth) Damage) 0.0 (CallFunction|GetMaxHealth))))

(event EventSetPlayerDead
  (params (ActorDead :type Boolean))
  (Variables|Default|SetbDead ActorDead))

(fn ControlEnemyLogic
  (params (Stop :type Boolean))
  (bind _returnvalue (Components|GetOwner))
  (bind _returnvalue_2 (AI|GetAIController _returnvalue))
  (bind _braincomponent (Variables|/Script/AIModule.AIController|GetBrainComponent _returnvalue_2))
  (if Stop
    (Utilities|IsValid _returnvalue_2
      (:Is%20Valid
        (Utilities|IsValid _braincomponent
          (:Is%20Valid
            (AI|Logic|StopLogic _braincomponent "Being Attacked")
            (CallFunction|StopMovementandAvoidance true)))))
    (else
      (Utilities|IsValid _returnvalue_2
        (:Is%20Valid
          (Utilities|IsValid _braincomponent
            (:Is%20Valid
              (AI|Logic|StartLogic _braincomponent)
              (CallFunction|StopMovementandAvoidance false))))))))

(fn StopMovementandAvoidance
  (params (Stop :type Boolean))
  (bind _returnvalue (Components|GetOwner))
  (bind _returnvalue_2 (Actor|GetComponentbyClass _returnvalue "/Script/Engine.CharacterMovementComponent"))
  (Utilities|IsValid _returnvalue_2
    (:Is%20Valid
      (Class|CharacterMovementComponent|SetAvoidanceEnabled _returnvalue_2 (not Stop)))))

(fn GetEnemyTeleportLocation
  (params (Offset :type Float%20%28double-precision%29))
  (bind _returnvalue (Components|GetOwner))
  (bind _returnvalue_2 (Components|GetOwner))
  (bind _returnvalue_3 (Utilities|Name|MakeLiteralName "TargetActor"))
  (bind _returnvalue_4 (Transformation|GetActorLocation _returnvalue_2))
  (bind _returnvalue_5 (AI|GetBlackboard _returnvalue))
  (bind _returnvalue_6 (AI|Components|Blackboard|GetValueasObject _returnvalue_5 _returnvalue_3))
  (bind _ascharacter (Utilities|Casting|CastToCharacter _returnvalue_6))
  (bind _returnvalue_7 (Transformation|GetActorLocation _ascharacter))
  (return (+ (* (Math|Vector|Normalize (- _returnvalue_4 _returnvalue_7)) Offset) _returnvalue_7) (Math|Rotator|FindLookatRotation _returnvalue_4 _returnvalue_7)))

(fn SetAttackPlayer
  (params (AttackPlayer :type Boolean))
  (bind _returnvalue (Components|GetOwner))
  (bind _returnvalue_2 (Components|GetOwner))
  (bind _returnvalue_3 (Utilities|Name|MakeLiteralName "TargetActor"))
  (bind _returnvalue_4 (AI|GetBlackboard _returnvalue_2))
  (bind _returnvalue_5 (AI|Components|Blackboard|GetValueasObject _returnvalue_4 _returnvalue_3))
  (bind _ascharacter (Utilities|Casting|CastToCharacter _returnvalue_5))
  (bind _returnvalue_6 (Actor|GetComponentbyClass _ascharacter "/Game/FFCS/Blueprints/Component/AC_FFCC.AC_FFCC_C"))
  (bind _output_get (Variables|Default|SetAttackingPlayer AttackPlayer))
  (if _output_get
    (Utilities|IsValid _returnvalue_4
      (:Is%20Valid
        (bind _output_get_2 (LocalVariables|SetAIState "Attack"))
        (AI|Components|Blackboard|SetValueasEnum _returnvalue_4 (Utilities|Name|MakeLiteralName "AIState") _output_get_2)
        (Utilities|IsValid _returnvalue_6
          (:Is%20Valid
            (Class|ACFFCCBase|SetCounterEnemy _returnvalue_6 _returnvalue)
            (Development|PrintString (Utilities|GetDisplayName _returnvalue) true true "(R=1.000000,G=0.000000,B=0.006518,A=1.000000)" 5.0))))
      (:Is%20Not%20Valid
        _)))
  (return))

(fn GetAttackPlayer
  (return (Variables|Default|GetAttackingPlayer)))

(fn HitDirection
  (params (Instigator :type Actor%20Object%20Reference))
  (bind _returnvalue (Transformation|GetActorLocation Instigator))
  (bind _returnvalue_2 (Components|GetOwner))
  (bind _returnvalue_3 (Transformation|GetActorLocation _returnvalue_2))
  (bind _returnvalue_4 (Transformation|GetActorRotation _returnvalue_2))
  (bind _returnvalue_5 (Math|Rotator|FindLookatRotation _returnvalue_3 _returnvalue))
  (bind _returnvalue_6 (Math|Rotator|Delta(Rotator) _returnvalue_5 _returnvalue_4))
  (if (Math|Float|InRange(Float) (.yaw _returnvalue_6) -45.0 45.0)
    (Development|PrintString "Forward" true true "(R=1.000000,G=0.000000,B=0.124302,A=1.000000)")
    (return "Fwd")
    (elif (Math|Float|InRange(Float) (.yaw _returnvalue_6) 45.0 135.0)
      (Development|PrintString "Right" true true "(R=1.000000,G=0.000000,B=0.124772,A=1.000000)")
      (return "Rt")
      (elif (or (Math|Float|InRange(Float) (.yaw _returnvalue_6) 135.0 1.8e+02) (Math|Float|InRange(Float) (.yaw _returnvalue_6) -179.99 -135.0))
        (Development|PrintString "Back" true true "(R=1.000000,G=0.000000,B=0.124772,A=1.000000)")
        (return "Bwd")
        (else
          (Development|PrintString "Left" true true "(R=1.000000,G=0.000000,B=0.124772,A=1.000000)")
          (return "Lt"))))))

(fn SetAIStatetoRandom
  (bind _returnvalue (Components|GetOwner))
  (bind _returnvalue_2 (AI|GetBlackboard _returnvalue))
  (Utilities|IsValid _returnvalue_2
    (:Is%20Valid
      (AI|Components|Blackboard|SetValueasEnum _returnvalue_2 (Utilities|Name|MakeLiteralName "AIState") (.OutItem (Utilities|Array|Random (Utilities|Array|MakeArray "GetInRange" "GetBack" "LookForWeapons" "Strafe")))))))

(fn ResetCounteredEnemyinPlayer
  (bind _returnvalue (Components|GetOwner))
  (bind _returnvalue_2 (Utilities|Name|MakeLiteralName "TargetActor"))
  (bind _returnvalue_3 (AI|GetBlackboard _returnvalue))
  (bind _returnvalue_4 (AI|Components|Blackboard|GetValueasObject _returnvalue_3 _returnvalue_2))
  (Utilities|IsValid _returnvalue_3
    (:Is%20Valid
      (Utilities|IsValid _returnvalue_4
        (:Is%20Valid
          (bind _ascharacter (Utilities|Casting|CastToCharacter _returnvalue_4))
          (Utilities|IsValid (Actor|GetComponentbyClass _ascharacter "/Game/FFCS/Blueprints/Component/AC_FFCC.AC_FFCC_C")
            (:Is%20Valid
              (Class|ACFFCCBase|SetCounterEnemy (Actor|GetComponentbyClass _ascharacter "/Game/FFCS/Blueprints/Component/AC_FFCC.AC_FFCC_C")))))
        (:Is%20Not%20Valid
          (Development|PrintString "Target retrieved failed" true true "(R=1.000000,G=0.000000,B=0.155774,A=1.000000)" :!label _label))))
    (:Is%20Not%20Valid
      (goto _label))))

(fn CheckCurrentandCounterEnemies
  (bind _returnvalue (Components|GetOwner))
  (bind _returnvalue_2 (Utilities|Name|MakeLiteralName "TargetActor"))
  (bind _returnvalue_3 (AI|GetBlackboard _returnvalue))
  (bind _returnvalue_4 (AI|Components|Blackboard|GetValueasObject _returnvalue_3 _returnvalue_2))
  (Utilities|IsValid _returnvalue_3
    (:Is%20Valid
      (Utilities|IsValid _returnvalue_4
        (:Is%20Valid
          (bind _ascharacter (Utilities|Casting|CastToCharacter _returnvalue_4))
          (Utilities|IsValid (Actor|GetComponentbyClass _ascharacter "/Game/FFCS/Blueprints/Component/AC_FFCC.AC_FFCC_C")
            (:Is%20Valid
              (return (== (Class|ACFFCCBase|GetCurrentEnemy (Actor|GetComponentbyClass _ascharacter "/Game/FFCS/Blueprints/Component/AC_FFCC.AC_FFCC_C")) (Class|ACFFCCBase|GetCounterEnemy (Actor|GetComponentbyClass _ascharacter "/Game/FFCS/Blueprints/Component/AC_FFCC.AC_FFCC_C")))))
            (:Is%20Not%20Valid
              (return false))))))))

(fn GetHealth
  (return (Variables|Default|GetCurrentHealth)))

(fn GetMaxHealth
  (return (Variables|Default|GetMaxHealth)))

(fn GetPlayerDead
  (return (Variables|Default|GetbDead)))