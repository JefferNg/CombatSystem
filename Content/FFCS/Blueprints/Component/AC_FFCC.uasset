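; Player free-flow combat component that holds state tag, health, current and counter enemies, animation sets, combo count and finisher readiness.
; Combo hits restart a timeout timer, and every tenth arms the finisher; being hit plays a directional montage and effect, resets the combo and damages the player.
; Tick runs medium and large cooldowns, pushed with combo state to the HUD.
; Helpers classify hit direction by yaw and pick montages by enemy distance.
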(event EventBeginPlay)

(event EventTick
  (params (DeltaSeconds :type Float%20%28single-precision%29))
  (bind _hud_ref (Variables|Default|GetHUD%20Ref))
  (bind _hud_ref_2 (Variables|Default|GetHUD%20Ref))
  (bind _uihudref (Variables|/Game/FFCS/Blueprints/HUD/BP_HUD_Main.BP_HUD_Main_C|GetUIHUDRef _hud_ref))
  (bind _uihudref_2 (Variables|/Game/FFCS/Blueprints/HUD/BP_HUD_Main.BP_HUD_Main_C|GetUIHUDRef _hud_ref_2))
  (Utilities|FlowControl|Sequence
    (:then_0
      (if (Variables|Default|GetLargeCoolDown)
        (Default|SetLargeCoolDown _uihudref_2 (Math|Float|Clamp(Float) (Variables|Default|GetCurrentLargeTimer) 0.0 (Variables|Default|GetLargeTimer)))
        (if (>= (Variables|Default|GetCurrentLargeTimer) (Variables|Default|GetLargeTimer))
          (Variables|Default|SetLargeCoolDown false)
          (Variables|Default|SetCurrentLargeTimer 0.0)
          (else
            (Variables|Default|SetCurrentLargeTimer (+ (Variables|Default|GetCurrentLargeTimer) DeltaSeconds))
            (Default|SetLargeTextColor (Variables|/Game/FFCS/Blueprints/HUD/BP_HUD_Main.BP_HUD_Main_C|GetUIHUDRef (Variables|Default|GetHUD%20Ref)) (Utilities|Struct|MakeSlateColor "(R=1.000000,G=1.000000,B=1.000000,A=1.000000)") "(R=1.000000,G=1.000000,B=1.000000,A=1.000000)")))
        (else
          (Default|SetLargeTextColor _uihudref_2 (Utilities|Struct|MakeSlateColor "(R=0.346704,G=0.000000,B=1.000000,A=1.000000)") "(R=0.345098,G=0.000000,B=1.000000,A=1.000000)"))))
    (:then_1
      (if (Variables|Default|GetMediumCoolDown)
        (Default|SetMediumCoolDown _uihudref (Math|Float|Clamp(Float) (Variables|Default|GetCurrentMediumTimer) 0.0 (Variables|Default|GetMediumTimer)))
        (if (>= (Variables|Default|GetCurrentMediumTimer) (Variables|Default|GetMediumTimer))
          (Variables|Default|SetMediumCoolDown false)
          (Variables|Default|SetCurrentMediumTimer 0.0)
          (else
            (Variables|Default|SetCurrentMediumTimer (+ (Variables|Default|GetCurrentMediumTimer) DeltaSeconds))
            (Default|SetMediumTextColor (Variables|/Game/FFCS/Blueprints/HUD/BP_HUD_Main.BP_HUD_Main_C|GetUIHUDRef (Variables|Default|GetHUD%20Ref)) (Utilities|Struct|MakeSlateColor "(R=1.000000,G=1.000000,B=1.000000,A=1.000000)") "(R=1.000000,G=1.000000,B=1.000000,A=1.000000)")))
        (else
          (Default|SetMediumTextColor _uihudref (Utilities|Struct|MakeSlateColor "(R=0.054480,G=1.000000,B=0.000000,A=1.000000)") "(R=0.054902,G=1.000000,B=0.000000,A=1.000000)"))))))

(event EventSetCounterAnims
  (params (NewCounterAnim :type Finisher%20Anim%20Data%20Structure%20%28by%20ref%29))
  (Variables|Default|SetCounterAnims NewCounterAnim))

(event EventSetMediumCoolDown
  (params (Delay :type Float%20%28single-precision%29))
  (Variables|Default|SetMediumTimer Delay)
  (Variables|Default|SetMediumCoolDown true))

(event EventSetLargeCoolDown
  (params (Delay :type Float%20%28single-precision%29))
  (Variables|Default|SetLargeTimer Delay)
  (Variables|Default|SetLargeCoolDown true))

(event EventPlayHitMontage
  (params (HitDirection :type EAttackHitDirection%20Enum :default "Fwd"))
  (bind _returnvalue (CallFunction|GetCurrentEnemy))
  (bind _returnvalue_2 (Components|GetOwner))
  (bind _returnvalue_3 (AI|GetAIController _returnvalue))
  (bind _returnvalue_4 (Actor|GetComponentbyClass _returnvalue_2 "/Script/Engine.MeshComponent"))
  (bind _returnvalue_5 (Actor|GetComponentbyClass _returnvalue_2 "/Script/Engine.SkeletalMeshComponent"))
  (bind _returnvalue_6 (Actor|GetComponentbyClass _returnvalue "/Game/FFCS/Blueprints/Component/AC_EnemyComp.AC_EnemyComp_C"))
  (Utilities|IsValid _returnvalue_5
    (:Is%20Valid
      (Utilities|IsValid _returnvalue_4
        (:Is%20Valid
          (Niagara|SpawnSystemAttached "/Game/Emitters/NS_HitEffect_System.NS_HitEffect_System" _returnvalue_4 "spine_02" "0, 0, 0" "0, 0, 0" "KeepRelativeOffset" true)
          (Animation|Montage|PlayMontage _returnvalue_5 (Utilities|Select :Index HitDirection :Fwd "/Game/FFCS/Blueprints/Animation/AM_Vic_1.AM_Vic_1" :Bwd "/Game/FFCS/Blueprints/Animation/MixamoUE4Model/AM_Vic_2.AM_Vic_2" :Lt "/Game/FFCS/Blueprints/Animation/MixamoUE4Model/AM_Vic_3.AM_Vic_3" :Rt "/Game/FFCS/Blueprints/Animation/MixamoUE4Model/AM_Vic_4.AM_Vic_4")
            (:then
              (Class|ACFFCCBase|ResetComboCounter)
              (CallFunction|SetTag (GameplayTags|MakeLiteralGameplayTag "(TagName=\"PlayerStates.HitReact\")"))
              (Utilities|IsValid _returnvalue
                (:Is%20Valid
                  (Utilities|IsValid _returnvalue_6
                    (:Is%20Valid
                      (Utilities|IsValid _returnvalue_3
                        (:Is%20Valid
                          (Default|ControlEnemyLogic _returnvalue_6 true)
                          (Game|Damage|ApplyDamage (Game|GetPlayerCharacter 0) 1e+01 _returnvalue_3 _returnvalue))))))))
            (:OnCompleted
              (CallFunction|SetTag (GameplayTags|MakeLiteralGameplayTag "(TagName=\"PlayerStates.Idle\")")))))))))

(event EventSetCurrentEnemy
  (params (EnemyRef :type Actor%20Object%20Reference))
  (bind _output_get (Variables|Default|SetCurrentEnemy EnemyRef))
  (Utilities|IsValid _output_get
    (:Is%20Valid
      (Utilities|IsValid (Actor|GetComponentbyClass (Variables|Default|GetCurrentEnemy) "/Game/FFCS/Blueprints/Component/AC_EnemyComp.AC_EnemyComp_C")
        (:Is%20Valid
          (Default|ControlEnemyLogic (Actor|GetComponentbyClass (Variables|Default|GetCurrentEnemy) "/Game/FFCS/Blueprints/Component/AC_EnemyComp.AC_EnemyComp_C") true))))))

(event EventSetCounterEnemy
  (params (EnemyRef :type Actor%20Object%20Reference))
  (Variables|Default|SetCounterEnemy EnemyRef))

(event EventSetHealth
  (params (Damage :type Float%20%28single-precision%29%20%28by%20ref%29))
  (Variables|Default|SetCurrentHealth (Math|Float|Clamp(Float) (- (CallFunction|GetHealth) Damage) 0.0 (CallFunction|GetMaxHealth))))

(event EventComboCounter
  (bind _hud_ref (Variables|Default|GetHUD%20Ref))
  (bind _uihudref (Variables|/Game/FFCS/Blueprints/HUD/BP_HUD_Main.BP_HUD_Main_C|GetUIHUDRef _hud_ref))
  (Utilities|FlowControl|Sequence
    (:then_0
      (bind _result (Math|Integer|IncrementInt (Variables|Default|GetCounter))
        (:%20%20
          (Default|SetCounterValue _uihudref _result)
          (Default|SetCounterVisibility _uihudref "Visible" 0.1)
          (Utilities|Time|ClearandInvalidateTimerbyHandle (Variables|Default|GetComboCounter_Timer))
          (bind _returnvalue (Utilities|Time|SetTimerbyEvent (EventDispatchers|CreateEvent :!event ResetComboCounter) 5.0))
          (Variables|Default|SetComboCounter_Timer _returnvalue)
          (if (== (Math|Integer|%(Integer) (Variables|Default|GetCounter) 10) 0)
            (CallFunction|SetFinisher true)
            (elif (not (CallFunction|GetFinisher))
              (CallFunction|SetFinisher false))))))
    (:then_1
      (Default|SetPercent _uihudref (Math|Conversions|ToFloat(Integer) _result)))))

(event EventResetComboCounter
  (bind _hud_ref (Variables|Default|GetHUD%20Ref))
  (bind _uihudref (Variables|/Game/FFCS/Blueprints/HUD/BP_HUD_Main.BP_HUD_Main_C|GetUIHUDRef _hud_ref))
  (bind _output_get (Variables|Default|SetCounter 0))
  (CallFunction|SetFinisher false)
  (Default|SetCounterValue _uihudref)
  (Default|SetCounterVisibility _uihudref "Collapsed" 2.0)
  (Default|SetPercent _uihudref (Math|Conversions|ToFloat(Integer) _output_get)))

(event EventSetFinisherAnims
  (params (NewFinisherData :type Finisher%20Anim%20Data%20Structure))
  (Variables|Default|SetFinisherAnims NewFinisherData))

(event EventSetAttackAnims
  (params (NewAttackAnim :type Player%20Attack%20Anim%20Data%20Structure%20%28by%20ref%29))
  (Variables|Default|SetAttackAnims NewAttackAnim))

(fn GetCurrentTag
  (return (Variables|Default|GetPlayerStateTag)))

(fn GetMontageonDistance
  (bind _returnvalue (Components|GetOwner))
  (bind _returnvalue_2 (CallFunction|GetCurrentEnemy))
  (bind _returnvalue_3 (Transformation|GetActorLocation _returnvalue_2))
  (bind _returnvalue_4 (Transformation|GetActorLocation _returnvalue))
  (bind _returnvalue_5 (Math|Vector|Distance(Vector) _returnvalue_3 _returnvalue_4))
  (if (Math|Float|InRange(Float) _returnvalue_5 0.0 (Utilities|Array|Get(acopy) (Variables|Setup|GetDistance)))
    (return (Variables|Setup|GetCloseCombatMontage))
    (elif (Math|Float|InRange(Float) _returnvalue_5 (Utilities|Array|Get(acopy) (Variables|Setup|GetDistance)) (Utilities|Array|Get(acopy) (Variables|Setup|GetDistance) 1))
      (return (Variables|Setup|GetMidRangeCombatMontage))
      (else
        (return (Variables|Setup|GetJumpCombatMontage))))))

(fn HitDirection
  (params (Instigator :type Actor%20Object%20Reference))
  (bind _returnvalue (Transformation|GetActorLocation Instigator))
  (bind _returnvalue_2 (Components|GetOwner))
  (bind _returnvalue_3 (Transformation|GetActorLocation _returnvalue_2))
  (bind _returnvalue_4 (Transformation|GetActorRotation _returnvalue_2))
  (bind _returnvalue_5 (Math|Rotator|FindLookatRotation _returnvalue_3 _returnvalue))
  (bind _returnvalue_6 (Math|Rotator|Delta(Rotator) _returnvalue_5 _returnvalue_4))
  (if (Math|Float|InRange(Float) (.yaw _returnvalue_6) -45.0 45.0)
    (Development|PrintString "Forward" true true "(R=1.000000,G=0.000000,B=0.124302,A=1.000000)")
    (return "Fwd")
    (elif (Math|Float|InRange(Float) (.yaw _returnvalue_6) 45.0 135.0)
      (Development|PrintString "Right" true true "(R=1.000000,G=0.000000,B=0.124772,A=1.000000)")
      (return "Rt")
      (elif (or (Math|Float|InRange(Float) (.yaw _returnvalue_6) 135.0 1.8e+02) (Math|Float|InRange(Float) (.yaw _returnvalue_6) -179.99 -135.0))
        (Development|PrintString "Back" true true "(R=1.000000,G=0.000000,B=0.124772,A=1.000000)")
        (return "Bwd")
        (else
          (Development|PrintString "Left" true true "(R=1.000000,G=0.000000,B=0.124772,A=1.000000)")
          (return "Lt"))))))

(fn GetCurrentEnemy
  (return (Variables|Default|GetCurrentEnemy)))

(fn SetTag
  (params (Tag :type Gameplay%20Tag%20Structure%20%28by%20ref%29))
  (Variables|Default|SetPlayerStateTag Tag)
  (return))

(fn GetTag
  (return (Variables|Default|GetPlayerStateTag)))

(fn GetCounterEnemy
  (return (Variables|Default|GetCounterEnemy)))

(fn GetDistancefromCounterEnemy
  (return (> (Transformation|GetDistanceTo (Components|GetOwner) (CallFunction|GetCounterEnemy)) (Variables|Default|GetTeleportDistance))))

(fn GetHUD
  (return (Variables|Default|GetHUD%20Ref)))

(fn SetHUD
  (params (HUD%20Ref :type BP%20HUD%20Main%20Object%20Reference))
  (Variables|Default|SetHUD%20Ref HUD%20Ref))

(fn SetFinisher
  (params (Finisher :type Boolean))
  (bind _hud_ref (Variables|Default|GetHUD%20Ref))
  (bind _uihudref (Variables|/Game/FFCS/Blueprints/HUD/BP_HUD_Main.BP_HUD_Main_C|GetUIHUDRef _hud_ref))
  (bind _output_get (Variables|Default|SetFinisher Finisher))
  (if _output_get
    (Default|SetCounterTextColor _uihudref "(R=1.000000,G=0.614453,B=0.050000,A=1.000000)")
    (Default|SetFinisherTextColor _uihudref (Utilities|Struct|MakeSlateColor "(R=1.000000,G=0.617207,B=0.049707,A=1.000000)") "(R=1.000000,G=0.617207,B=0.049707,A=1.000000)")
    (else
      (Default|SetCounterTextColor _uihudref "(R=1.000000,G=1.000000,B=1.000000,A=1.000000)")
      (Default|SetFinisherTextColor _uihudref (Utilities|Struct|MakeSlateColor "(R=1.000000,G=1.000000,B=1.000000,A=1.000000)") "(R=1.000000,G=1.000000,B=1.000000,A=1.000000)"))))

(fn GetFinisher
  (return (Variables|Default|GetFinisher)))

(fn GetFinisherAnims
  (return (Variables|Default|GetFinisherAnims)))

(fn GetAttackAnims
  (return (Variables|Default|GetAttackAnims)))

(fn GetCounterAnims
  (return (Variables|Default|GetCounterAnims)))

(fn GetHealth
  (return (Variables|Default|GetCurrentHealth)))

(fn GetMaxHealth
  (return (Variables|Default|GetMaxHealth)))