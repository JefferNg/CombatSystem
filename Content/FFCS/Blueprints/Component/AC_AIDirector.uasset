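; AI director component that paces enemy attacks on its owner, allowing one attacker at a time.
; AddEnemy and RemoveEnemy maintain the enemy list, starting a randomized-interval looping timer and clearing it once the list empties.
; Each check skips while the owner's AC_FFCC has a counter enemy or Finisher tag.
; Otherwise, if no living enemy is attacking, it flags a randomly picked one through AC_EnemyComp.
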(event EventBeginPlay)

(event EventTick
  (params (DeltaSeconds :type Float%20%28single-precision%29)))

(fn AddEnemy
  (params (EnemyRef :type Actor%20Object%20Reference))
  (bind _enemy_ref (Variables|Default|GetEnemy%20Ref))
  (Utilities|Array|AddUnique _enemy_ref EnemyRef)
  (if (and (not (Utilities|Time|IsTimerActivebyHandle (Variables|Default|GetCheckAttackPlayerTH))) (> (Utilities|Array|Length _enemy_ref) 0))
    (bind _returnvalue (Utilities|Time|SetTimerbyFunctionName 0 "CheckIfPlayerUnderAttack" (Math|Random|RandomFloatinRange 5.0 8.0) true))
    (Variables|Default|SetCheckAttackPlayerTH _returnvalue)))

(fn RemoveEnemy
  (params (EnemyRef :type Actor%20Object%20Reference))
  (bind _enemy_ref (Variables|Default|GetEnemy%20Ref))
  (Utilities|Array|RemoveItem _enemy_ref EnemyRef)
  (if (<= (Utilities|Array|Length _enemy_ref) 0)
    (Utilities|Time|ClearandInvalidateTimerbyHandle (Variables|Default|GetCheckAttackPlayerTH))))

(fn CheckifPlayerUnderAttack
  (bind _returnvalue (Components|GetOwner))
  (bind _enemy_ref (Variables|Default|GetEnemy%20Ref))
  (bind _outitem (Utilities|Array|Random _enemy_ref))
  (bind _returnvalue_2 (Actor|GetComponentbyClass _returnvalue "/Game/FFCS/Blueprints/Component/AC_FFCC.AC_FFCC_C"))
  (bind _returnvalue_3 (Actor|GetComponentbyClass _outitem "/Game/FFCS/Blueprints/Component/AC_EnemyComp.AC_EnemyComp_C"))
  (Utilities|IsValid _returnvalue_2
    (:Is%20Valid
      (Utilities|IsValid (Class|ACFFCCBase|GetCounterEnemy _returnvalue_2)
        (:Is%20Not%20Valid
          (if (GameplayTags|MatchesAnyTags (Class|ACFFCCBase|GetTag _returnvalue_2) (GameplayTags|MakeLiteralGameplayTagContainer "(GameplayTags=((TagName=\"PlayerStates.Finisher\"),(TagName=\"PlayerStates.FinisherInProgress\")))"))
            (Development|PrintString "Finisher active")
            (else
              (LocalVariables|SetChooseAIToAttack true :!label _label)
              (for _array_element (Variables|Default|GetEnemy%20Ref)
                (Utilities|IsValid (Actor|GetComponentbyClass _array_element "/Game/FFCS/Blueprints/Component/AC_EnemyComp.AC_EnemyComp_C")
                  (:Is%20Valid
                    (if (and (not (Variables|/Script/FreeFlowCombatSystem.AC_EnemyComp_Base|GetbDead (Actor|GetComponentbyClass _array_element "/Game/FFCS/Blueprints/Component/AC_EnemyComp.AC_EnemyComp_C"))) (Class|ACEnemyCompBase|GetAttackPlayer (Actor|GetComponentbyClass _array_element "/Game/FFCS/Blueprints/Component/AC_EnemyComp.AC_EnemyComp_C")))
                      (LocalVariables|SetChooseAIToAttack false)))))
              (if (LocalVariables|GetChooseAIToAttack)
                (Utilities|IsValid _outitem
                  (:Is%20Valid
                    (Utilities|IsValid _returnvalue_3
                      (:Is%20Valid
                        (if (not (Variables|/Script/FreeFlowCombatSystem.AC_EnemyComp_Base|GetbDead _returnvalue_3))
                          (Class|ACEnemyCompBase|SetAttackPlayer _returnvalue_3 true))))))))))))
    (:Is%20Not%20Valid
      (goto _label))))