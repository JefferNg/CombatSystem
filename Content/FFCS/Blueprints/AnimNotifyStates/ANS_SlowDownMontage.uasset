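; Anim notify state that slows or re-times the active montage during its window, apparently for AI attacks that can be countered.
; Begin applies NewPlayRate to the current montage and end applies ResetPlayRate.
; Tick reads TargetActor from the owner's blackboard and checks its AC_FFCC component for the exact PlayerStates.Countered tag.
; A match stops the montage once with a blend-out, using a DoOnce that resets when the tag differs.
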(fn ReceivedNotifyBegin
  (params (MeshComp :type Skeletal%20Mesh%20Component%20Object%20Reference) (Animation :type Anim%20Sequence%20Base%20Object%20Reference) (TotalDuration :type Float%20%28single-precision%29) (EventReference :type Anim%20Notify%20Event%20Reference%20Structure%20%28by%20ref%29))
  (bind _returnvalue (Components|SkeletalMesh|GetAnimInstance MeshComp))
  (Animation|Montage|MontageSetPlayRate _returnvalue (Animation|Montage|GetCurrentActiveMontage _returnvalue) (Variables|Default|GetNewPlayRate))
  (return false))

(fn ReceivedNotifyEnd
  (params (MeshComp :type Skeletal%20Mesh%20Component%20Object%20Reference) (Animation :type Anim%20Sequence%20Base%20Object%20Reference) (EventReference :type Anim%20Notify%20Event%20Reference%20Structure%20%28by%20ref%29))
  (bind _returnvalue (Components|SkeletalMesh|GetAnimInstance MeshComp))
  (Animation|Montage|MontageSetPlayRate _returnvalue (Animation|Montage|GetCurrentActiveMontage _returnvalue) (Variables|Default|GetResetPlayRate))
  (return false))

(fn ReceivedNotifyTick
  (params (MeshComp :type Skeletal%20Mesh%20Component%20Object%20Reference) (Animation :type Anim%20Sequence%20Base%20Object%20Reference) (FrameDeltaTime :type Float%20%28single-precision%29) (EventReference :type Anim%20Notify%20Event%20Reference%20Structure%20%28by%20ref%29))
  (bind _returnvalue (Components|SkeletalMesh|GetAnimInstance MeshComp))
  (bind _returnvalue_2 (Utilities|Name|MakeLiteralName "TargetActor"))
  (bind _returnvalue_3 (Components|GetOwner MeshComp))
  (bind _returnvalue_4 (AI|GetBlackboard _returnvalue_3))
  (bind _returnvalue_5 (AI|Components|Blackboard|GetValueasObject _returnvalue_4 _returnvalue_2))
  (bind _ascharacter (Utilities|Casting|CastToCharacter _returnvalue_5))
  (bind _returnvalue_6 (Actor|GetComponentbyClass _ascharacter "/Game/FFCS/Blueprints/Component/AC_FFCC.AC_FFCC_C"))
  (Utilities|IsValid _returnvalue_4
    (:Is%20Valid
      (Utilities|IsValid _returnvalue_6
        (:Is%20Valid
          (if (GameplayTags|MatchesTag (Class|ACFFCCBase|GetTag _returnvalue_6) "(TagName=\"PlayerStates.Countered\")" true)
            (Utilities|FlowControl|DoOnce false :!label _label
              (:Completed
                (Animation|Montage|MontageStop _returnvalue 0.5 (Animation|Montage|GetCurrentActiveMontage _returnvalue))
                (return false)))
            (else
              (goto _label Reset))))))))