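; BP_Grunt is an AI enemy that detects the player and joins the player's AC_AIDirector enemy list.
; AIPerception sets the blackboard TargetActor, while a short timer delays clearing it and deregistering after sight is lost.
; AnyDamage feeds ACEnemyComp; at zero health the grunt leaves the director, stops its AI and strips core components.
; Tick turns the health bar toward the camera and labels the grunt while attacking.
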(event OnTargetPerceptionUpdated(AIPerception)
  (params (Actor :type Actor%20Object%20Reference) (Stimulus :type AI%20Stimulus%20Structure))
  (bind _returnvalue (Actor|GetComponentbyClass Actor "/Game/FFCS/Blueprints/Component/AC_AIDirector.AC_AIDirector_C"))
  (if (== Actor (Game|GetPlayerCharacter 0))
    (if (.bSuccessfullySensed (Utilities|Struct|BreakAIStimulus Stimulus))
      (Utilities|Time|ClearandInvalidateTimerbyHandle (Variables|Default|GetTargetCheckerTH))
      (Utilities|IsValid _returnvalue
        (:Is%20Valid
          (Default|AddEnemy _returnvalue self))
        (:Is%20Not%20Valid
          _))
      (AI|Components|Blackboard|SetValueasObject (AI|GetBlackboard 0) (Utilities|Name|MakeLiteralName "TargetActor") Actor)
      (else
        (bind _returnvalue_2 (Utilities|Time|SetTimerbyFunctionName 0 "CheckIfTargetLost" 2.0))
        (Variables|Default|SetTargetCheckerTH _returnvalue_2)))))

(event EventBeginPlay
  (|CallParentFunction))

(event Collision|EventActorBeginOverlap
  (params (OtherActor :type Actor%20Object%20Reference)))

(event EventTick
  (params (DeltaSeconds :type Float%20%28single-precision%29))
  (bind _healthbarwidget (Variables|Default|GetHealthBarWidget))
  (bind _ac_enemycomp (Variables|Default|GetAC_EnemyComp))
  (Utilities|FlowControl|Sequence
    (:then_0
      (bind _aswb_health_bar (Utilities|Casting|CastToWB_HealthBar (UserInterface|GetWidget _healthbarwidget)))
      (Utilities|IsValid _ac_enemycomp
        (:Is%20Valid
          (Progress|SetPercent (Variables|/Game/FFCS/Blueprints/UI/WB_HealthBar.WB_HealthBar_C|GetHealthBar _aswb_health_bar) (/ (Class|ACEnemyCompBase|GetHealth _ac_enemycomp) (Class|ACEnemyCompBase|GetMaxHealth _ac_enemycomp))))
        (:Is%20Not%20Valid
          (Progress|SetPercent (Variables|/Game/FFCS/Blueprints/UI/WB_HealthBar.WB_HealthBar_C|GetHealthBar _aswb_health_bar) 0.0)))
      (Transformation|SetWorldRotation _healthbarwidget (Math|Rotator|FindLookatRotation (Transformation|GetWorldLocation _healthbarwidget) (Transformation|GetWorldLocation (Variables|/Script/Engine.PlayerCameraManager|GetTransformComponent (Game|GetPlayerCameraManager 0)))) false false))
    (:then_1
      (bind _ac_enemycomp_2 (Variables|Default|GetAC_EnemyComp)
        (:then
          (Rendering|Components|TextRender|SetText (Variables|Default|GetTextRender) (Utilities|Text|ToText(String) (Utilities|String|SelectString (Utilities|String|ToString(Text) (Utilities|Text|ToText(String) (Utilities|String|Append "Attacking" (Utilities|GetDisplayName self)))) "" (Class|ACEnemyCompBase|GetAttackPlayer _ac_enemycomp_2)))))
        (:else)))))

(event Game|Damage|EventAnyDamage
  (params (Damage :type Float%20%28single-precision%29) (DamageType :type Damage%20Type%20Object%20Reference) (InstigatedBy :type Controller%20Object%20Reference) (DamageCauser :type Actor%20Object%20Reference))
  (bind _returnvalue (Actor|GetComponentbyClass DamageCauser "/Game/FFCS/Blueprints/Component/AC_AIDirector.AC_AIDirector_C"))
  (bind _ac_enemycomp (Variables|Default|GetAC_EnemyComp))
  (Class|ACEnemyCompBase|SetHealth _ac_enemycomp Damage)
  (if (<= (Class|ACEnemyCompBase|GetHealth _ac_enemycomp) 0.0)
    (Utilities|IsValid _returnvalue
      (:Is%20Valid
        (Default|RemoveEnemy _returnvalue self))
      (:Is%20Not%20Valid
        (bind _returnvalue_2 (Actor|GetActorOfClass "/Game/FFCS/Blueprints/Character/BP_Player.BP_Player_C"))
        (Default|RemoveEnemy (Variables|/Game/FFCS/Blueprints/Character/BP_Player.BP_Player_C|GetAC_AIDirector _returnvalue_2) self)))
    (Class|ACEnemyCompBase|SetPlayerDead _ac_enemycomp true)
    (AI|Logic|StopLogic (Variables|/Script/AIModule.AIController|GetBrainComponent (AI|GetAIController self)) "")
    (Class|Pawn|DetachfromControllerPendingDestroy)
    (Components|DestroyComponent (Variables|Character|GetCharacterMovement))
    (Components|DestroyComponent (Variables|Default|GetAC_EnemyComp))
    (Components|DestroyComponent (Variables|Default|GetAIPerception))
    (Collision|SetCollisionEnabled (Variables|Default|GetCapsuleComponent) "PhysicsOnly")
    (Variables|Default|SetIsDead true)))

(fn ConstructionScript
  (|CallParentFunction))

(fn CheckifTargetLost
  (bind _returnvalue (Utilities|Name|MakeLiteralName "TargetActor"))
  (bind _returnvalue_2 (AI|GetBlackboard 0))
  (bind _returnvalue_3 (AI|Components|Blackboard|GetValueasObject _returnvalue_2 _returnvalue))
  (bind _ascharacter (Utilities|Casting|CastToCharacter _returnvalue_3))
  (bind _returnvalue_4 (Actor|GetComponentbyClass _ascharacter "/Game/FFCS/Blueprints/Component/AC_AIDirector.AC_AIDirector_C"))
  (Utilities|IsValid _returnvalue_2
    (:Is%20Valid
      (Utilities|IsValid _returnvalue_3
        (:Is%20Valid
          (Utilities|IsValid _returnvalue_4
            (:Is%20Valid
              (Default|RemoveEnemy _returnvalue_4 self))
            (:Is%20Not%20Valid
              _))
          (AI|Components|Blackboard|SetValueasObject _returnvalue_2 _returnvalue 0))))))