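; AN_CounterHit is an animation notify that lands the hit of a counter attack on the enemy stored in the owner's AC_FFCC combat component.
; It advances the component's combo counter and applies damage, with player controller 0 as instigator.
; If the enemy has a mesh component, it attaches a Niagara hit effect at spine_02, clears the stored enemy and plays a 2D impact sound.
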(fn ReceivedNotify
  (params (MeshComp :type Skeletal%20Mesh%20Component%20Object%20Reference) (Animation :type Anim%20Sequence%20Base%20Object%20Reference) (EventReference :type Anim%20Notify%20Event%20Reference%20Structure%20%28by%20ref%29))
  (bind _returnvalue (Components|GetOwner MeshComp))
  (bind _returnvalue_2 (Actor|GetComponentbyClass _returnvalue "/Game/FFCS/Blueprints/Component/AC_FFCC.AC_FFCC_C"))
  (bind _returnvalue_3 (Class|ACFFCCBase|GetCounterEnemy _returnvalue_2))
  (bind _returnvalue_4 (Actor|GetComponentbyClass _returnvalue_3 "/Script/Engine.MeshComponent"))
  (Utilities|IsValid _returnvalue
    (:Is%20Valid
      (Utilities|IsValid _returnvalue_2
        (:Is%20Valid
          (Utilities|IsValid _returnvalue_3
            (:Is%20Valid
              (Class|ACFFCCBase|ComboCounter _returnvalue_2)
              (Game|Damage|ApplyDamage _returnvalue_3 (Variables|Default|GetBase%20Damage) (Game|GetPlayerController 0) _returnvalue)
              (Utilities|IsValid _returnvalue_4
                (:Is%20Valid
                  (Niagara|SpawnSystemAttached "/Game/Emitters/NS_HitEffect_System.NS_HitEffect_System" _returnvalue_4 "spine_02" "0, 0, 0" "0, 0, 0" "KeepRelativeOffset" true)
                  (Class|ACFFCCBase|SetCounterEnemy _returnvalue_2)
                  (Audio|PlaySound2D "/Game/Sounds/wet-snowball-hit-2.wet-snowball-hit-2" 1.0 1.0 0.0 0 0)
                  (return true))))))
        (:Is%20Not%20Valid
          _)))
    (:Is%20Not%20Valid
      _))
  (return false))