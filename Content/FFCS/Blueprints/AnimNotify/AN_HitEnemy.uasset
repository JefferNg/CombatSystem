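; Anim notify that lands the player's melee hit on the current enemy of the FFCS combat component (AC_FFCC).
; It only acts for BP_Player with a valid enemy that has AC_EnemyComp and a mesh, attaching a Niagara hit effect at spine_02.
; If a finisher is available, the player runs TeleportAndKill.
; Otherwise the enemy plays a directional hit montage, the combo counter is called and the attack's damage is applied.
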(fn ReceivedNotify
  (params (MeshComp :type Skeletal%20Mesh%20Component%20Object%20Reference) (Animation :type Anim%20Sequence%20Base%20Object%20Reference) (EventReference :type Anim%20Notify%20Event%20Reference%20Structure%20%28by%20ref%29))
  (bind _returnvalue (Components|GetOwner MeshComp))
  (bind _returnvalue_2 (Actor|GetComponentbyClass _returnvalue "/Game/FFCS/Blueprints/Component/AC_FFCC.AC_FFCC_C"))
  (bind _returnvalue_3 (Class|ACFFCCBase|GetCurrentEnemy _returnvalue_2))
  (bind _returnvalue_4 (Actor|GetComponentbyClass _returnvalue_3 "/Game/FFCS/Blueprints/Component/AC_EnemyComp.AC_EnemyComp_C"))
  (bind _returnvalue_5 (Actor|GetComponentbyClass _returnvalue_3 "/Script/Engine.MeshComponent"))
  (bind _asbp_player (Utilities|Casting|CastToBP_Player _returnvalue))
  (Utilities|IsValid _returnvalue_2
    (:Is%20Valid
      (Utilities|IsValid _returnvalue_3
        (:Is%20Valid
          (Utilities|IsValid _returnvalue_4
            (:Is%20Valid
              (Utilities|IsValid _returnvalue_5
                (:Is%20Valid
                  (Niagara|SpawnSystemAttached "/Game/Emitters/NS_HitEffect_System.NS_HitEffect_System" _returnvalue_5 "spine_02" "0, 0, 0" "0, 0, 0" "KeepRelativeOffset" true)
                  (bind _returnvalue_6 (Default|CanPlayFinisher _asbp_player))
                  (if _returnvalue_6
                    (Default|TeleportandKill _asbp_player)
                    (else
                      (bind _returnvalue_7 (Class|ACEnemyCompBase|HitDirection _returnvalue_4 _returnvalue))
                      (Default|PlayHitMontage _returnvalue_4 _returnvalue_7)
                      (Class|ACFFCCBase|ComboCounter _returnvalue_2)
                      (Game|Damage|ApplyDamage _returnvalue_3 (Utilities|Struct|BreakPlayerAttackAnimData (Variables|/Script/FreeFlowCombatSystem.AC_FFCC_Base|GetAttackAnims _returnvalue_2)) (Game|GetPlayerController 0) _returnvalue)
                      (return true))))))))))))